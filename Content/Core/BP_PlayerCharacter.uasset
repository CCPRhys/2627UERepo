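; Player character that moves and looks with Enhanced Input and can take control of vehicles.
; BeginPlay adds IMC_Main, and mouse look is scaled by MouseSens and delta time.
; Interact box-traces for a BP_Vehicle_Base pawn just ahead, with debug drawing, then calls PossessOnServer.
; That event repeats the trace, switches the controller to the vehicle and destroys the character, a step flagged "Don't do this".
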(event EventBeginPlay
  (Input|AddMappingContext (PlayerController|LocalPlayerSubsystems|GetEnhancedInputLocalPlayerSubsystem (Game|GetPlayerController 0)) "/Game/Inputs/IMC_Main.IMC_Main" 0 "(bIgnoreAllPressedKeysUntilRelease=True,bForceImmediately=False,bNotifyUserSettings=False)"))

(event Collision|EventActorBeginOverlap
  (params (OtherActor :type Actor%20Object%20Reference)))

(event EventTick
  (params (DeltaSeconds :type Float%20%28single-precision%29)))

(event Custom|PossessOnServer
  (params (Target :type Controller%20Object%20Reference))
  (bind _returnvalue (Transformation|GetActorLocation))
  (bind _returnvalue_2 (Transformation|GetActorForwardVector))
  (bind _returnvalue_3 (* _returnvalue_2 3e+01))
  (bind _returnvalue_4 (+ _returnvalue _returnvalue_3))
  (bind (_outhit _returnvalue_5) (Class|KismetSystemLibrary|BoxTraceSingleforObjects _returnvalue_4 _returnvalue_4 "100.000000,100.000000,100.000000" (Math|Conversions|RotationFromXVector _returnvalue_2) (Utilities|Array|MakeArray "ObjectTypeQuery3") false 0 "ForDuration" true))
  (if _returnvalue_5
    (bind _asbp_vehicle_base (Utilities|Casting|CastToBP_Vehicle_Base (.HitActor (Collision|BreakHitResult _outhit))))
    (Pawn|UnPossess Target)
    (Pawn|Possess Target _asbp_vehicle_base)
    ;[1 0 0.03447 0.5] Don't do this
    (Actor|DestroyActor)))

(event Input|EnhancedActionEvents|EnhancedInputActionIA_Movement
  (params (ActionValue :type Vector%202D%20Structure) (ElapsedSeconds :type Float%20%28double-precision%29) (TriggeredSeconds :type Float%20%28double-precision%29) (InputAction :type Input%20Action%20Object%20Reference :default "/Game/Inputs/IA_Movement.IA_Movement"))
  (bind (_x _y) (Math|Vector2D|BreakVector2D ActionValue))
  (Pawn|Input|AddMovementInput (Transformation|GetActorForwardVector) _y false)
  (Pawn|Input|AddMovementInput (Transformation|GetActorRightVector) _x false))

(event Input|EnhancedActionEvents|EnhancedInputActionIA_Mouse
  (params (ActionValue :type Vector%202D%20Structure) (ElapsedSeconds :type Float%20%28double-precision%29) (TriggeredSeconds :type Float%20%28double-precision%29) (InputAction :type Input%20Action%20Object%20Reference :default "/Game/Inputs/IA_Mouse.IA_Mouse"))
  (bind (_x _y) (Math|Vector2D|BreakVector2D ActionValue))
  (bind _returnvalue (Utilities|Time|GetWorldDeltaSeconds))
  (bind _mousesens (Variables|Default|GetMouseSens))
  (Pawn|Input|AddControllerYawInput (* _x _returnvalue _mousesens))
  (Pawn|Input|AddControllerPitchInput (* _y _returnvalue _mousesens)))

(event Input|EnhancedActionEvents|EnhancedInputActionIA_Interact
  (params (ActionValue :type Boolean) (ElapsedSeconds :type Float%20%28double-precision%29) (TriggeredSeconds :type Float%20%28double-precision%29) (InputAction :type Input%20Action%20Object%20Reference :default "/Game/Inputs/IA_Interact.IA_Interact"))
  (bind _returnvalue (Transformation|GetActorForwardVector))
  (bind _returnvalue_2 (Transformation|GetActorLocation))
  (bind _returnvalue_3 (* _returnvalue 3e+01))
  (bind _returnvalue_4 (+ _returnvalue_2 _returnvalue_3))
  (:Started
    (bind (_outhit _returnvalue_5) (Class|KismetSystemLibrary|BoxTraceSingleforObjects _returnvalue_4 _returnvalue_4 "100.000000,100.000000,100.000000" (Math|Conversions|RotationFromXVector _returnvalue) (Utilities|Array|MakeArray "ObjectTypeQuery3") false 0 "ForDuration" true))
    (if _returnvalue_5
      (Utilities|Casting|CastToBP_Vehicle_Base (.HitActor (Collision|BreakHitResult _outhit)))
      (CallFunction|PossessonServer (Game|GetPlayerController 0)))))

(fn ConstructionScript)