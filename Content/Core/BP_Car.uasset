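; BP_Car is a drivable vehicle pawn that the player can exit on foot.
; It adds the IMC_Main Enhanced Input mapping on BeginPlay, then drives forward and back with AddMovementInput and steers by frame-time-scaled controller yaw.
; The interact input spawns a new BP_PlayerCharacter beside the car, facing it, and switches player controller 0's possession to that character.
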(event EventBeginPlay
  (Input|AddMappingContext (PlayerController|LocalPlayerSubsystems|GetEnhancedInputLocalPlayerSubsystem (Game|GetPlayerController 0)) "/Game/Inputs/IMC_Main.IMC_Main" 0 "(bIgnoreAllPressedKeysUntilRelease=True,bForceImmediately=False,bNotifyUserSettings=False)"))

(event Collision|EventActorBeginOverlap
  (params (OtherActor :type Actor%20Object%20Reference)))

(event EventTick
  (params (DeltaSeconds :type Float%20%28single-precision%29)))

(event Input|EnhancedActionEvents|EnhancedInputActionIA_Movement
  (params (ActionValue :type Vector%202D%20Structure) (ElapsedSeconds :type Float%20%28double-precision%29) (TriggeredSeconds :type Float%20%28double-precision%29) (InputAction :type Input%20Action%20Object%20Reference :default "/Game/Inputs/IA_Movement.IA_Movement"))
  (bind (_x _y) (Math|Vector2D|BreakVector2D ActionValue))
  (Pawn|Input|AddMovementInput (Transformation|GetActorForwardVector) _y false)
  (Pawn|Input|AddControllerYawInput (* _x (Utilities|Time|GetWorldDeltaSeconds) (Variables|Default|GetTurnSpeed))))

(event Input|EnhancedActionEvents|EnhancedInputActionIA_Interact
  (params (ActionValue :type Boolean) (ElapsedSeconds :type Float%20%28double-precision%29) (TriggeredSeconds :type Float%20%28double-precision%29) (InputAction :type Input%20Action%20Object%20Reference :default "/Game/Inputs/IA_Interact.IA_Interact"))
  (bind _returnvalue (Transformation|GetActorRightVector))
  (:Started
    (bind _returnvalue_2 (Game|SpawnActorfromClass "/Game/Core/BP_PlayerCharacter.BP_PlayerCharacter_C" (Math|Transform|MakeTransform (+ (Transformation|GetActorLocation) (* _returnvalue 1e+02)) (Math|Conversions|RotationFromXVector (* _returnvalue -1.0)) "1.000000,1.000000,1.000000") "AdjustIfPossibleButAlwaysSpawn" "MultiplyWithRoot" 0 0))
    (Pawn|UnPossess (Game|GetPlayerController 0))
    (Pawn|Possess (Game|GetPlayerController 0) _returnvalue_2)))

(fn ConstructionScript)