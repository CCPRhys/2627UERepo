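; Vehicle Blueprint with a mouse-aimed turret that fires projectiles on a cooldown, built for networked play.
; Mouse input yaws the turret locally, mirrors the change to the server from clients, and aligns RotationPoint to the turret.
; Clients fire a local predicted projectile immediately, then route the shot through ShootOnServer to ShootOnEveryone.
; Non-local projectiles hide their Sphere from the owner to mask the duplicate, while Tick counts down the cooldown.
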(event Custom|Shoot
  (params (Owner :type Actor%20Object%20Reference) (Local :type Boolean))
  ;[0.15 0.15 0.15 0.5] Shoot
  (bind _offcooldown (CallFunction|CanShoot))
  (if _offcooldown
    (bind _returnvalue (Game|SpawnActorfromClass (Variables|Default|GetProjectileToShoot) (Math|Transform|MakeTransform (Transformation|GetWorldLocation (Variables|Default|GetShootPosition)) (Transformation|GetWorldRotation (Variables|Default|GetTurret)) "1.000000,1.000000,1.000000") "Undefined" "MultiplyWithRoot" Owner 0))
    (CallFunction|PutonCooldown)
    (if (not Local)
      (Class|PrimitiveComponent|SetOwnerNoSee (Variables|/Game/Projectiles/BP_Projectile_Base.BP_Projectile_Base_C|GetSphere _returnvalue) true))))

(event EventBeginPlay
  (|CallParentFunction) ; This node is disabled and will not be called.\nDrag off pins to build functionality.
)

(event Collision|EventActorBeginOverlap
  (params (OtherActor :type Actor%20Object%20Reference))
  (|CallParentFunction OtherActor) ; This node is disabled and will not be called.\nDrag off pins to build functionality.
)

(event EventTick
  (params (DeltaSeconds :type Float%20%28single-precision%29))
  (|CallParentFunction DeltaSeconds)
  (CallFunction|ReduceCooldown))

(event Custom|RotateOnServer
  (params (Amount :type Float%20%28double-precision%29))
  (Transformation|AddLocalRotation (Variables|Default|GetTurret) (Math|Rotator|MakeRotator 0.0 0.0 Amount) false false))

(event Custom|ShootOnServer
  (params (Owner :type Actor%20Object%20Reference) (Local :type Boolean))
  (CallFunction|ShootonEveryone Owner Local))

(event Custom|ShootOnEveryone
  (params (Owner :type Actor%20Object%20Reference) (Local :type Boolean))
  (CallFunction|Shoot Owner Local))

(event Input|EnhancedActionEvents|EnhancedInputActionIA_Mouse
  (params (ActionValue :type Vector%202D%20Structure) (ElapsedSeconds :type Float%20%28double-precision%29) (TriggeredSeconds :type Float%20%28double-precision%29) (InputAction :type Input%20Action%20Object%20Reference :default "/Game/Inputs/IA_Mouse.IA_Mouse"))
  (bind _x (Math|Vector2D|BreakVector2D ActionValue))
  (bind _returnvalue (Utilities|Time|GetWorldDeltaSeconds))
  (bind _turretspeed (Variables|Default|GetTurretSpeed))
  (bind _returnvalue_2 (* _x _returnvalue _turretspeed))
  (Networking|SwitchHasAuthority
    (:Authority
      _)
    (:Remote
      (CallFunction|RotateonServer _returnvalue_2)))
  (Transformation|AddLocalRotation (Variables|Default|GetTurret) (Math|Rotator|MakeRotator 0.0 0.0 _returnvalue_2) false false)
  (Transformation|SetWorldRotation (Variables|Default|GetRotationPoint) (Transformation|GetWorldRotation (Variables|Default|GetTurret)) false false))

(event Input|EnhancedActionEvents|EnhancedInputActionIA_Shoot
  (params (ActionValue :type Boolean) (ElapsedSeconds :type Float%20%28double-precision%29) (TriggeredSeconds :type Float%20%28double-precision%29) (InputAction :type Input%20Action%20Object%20Reference :default "/Game/Inputs/IA_Shoot.IA_Shoot"))
  (bind _self self)
  (Networking|SwitchHasAuthority
    (:Authority
      (CallFunction|ShootonEveryone _self true))
    (:Remote
      (CallFunction|Shoot _self true)
      (CallFunction|ShootonServer _self false))))

(fn ConstructionScript
  (|CallParentFunction))

(fn CanShoot
  (return (== (Variables|Default|Getcooldown) 0.0)))

(fn ReduceCooldown
  (Variables|Default|Setcooldown (Math|Float|Clamp(Float) (- (Variables|Default|Getcooldown) (Utilities|Time|GetWorldDeltaSeconds)) 0.0 (Variables|Default|GetCooldownMax))))

(fn PutonCooldown
  (Variables|Default|Setcooldown (Variables|Default|GetCooldownMax)))