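; BP_Tank is a tank Blueprint that shows its controlling player's team colour on the turret and barrel.
; BeginPlay creates and stores dynamic instances of M_TeamColour for both meshes, whose Colour parameter ChangeTeamColour updates.
; On possession by a BP_PC, it applies that controller's TeamColour and adds a BP_Test widget to the viewport.
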(event Custom|ChangeTeamColour
  (params (Colour :type Linear%20Color%20Structure))
  (Variables|Default|SetTeamColour Colour)
  (Rendering|Material|SetVectorParameterValue (Variables|Default|GetTurretMaterial) "Colour" (Variables|Default|GetTeamColour) :!class /Script/Engine.MaterialInstanceDynamic)
  (Rendering|Material|SetVectorParameterValue (Variables|Default|GetBarrelMaterial) "Colour" (Variables|Default|GetTeamColour) :!class /Script/Engine.MaterialInstanceDynamic))

(event EventBeginPlay
  (|CallParentFunction)
  (bind _returnvalue (Rendering|Material|CreateDynamicMaterialInstance (Variables|Default|GetTurret) 0 "/Game/Art/3D/M_TeamColour.M_TeamColour" "None" :!class /Script/Engine.PrimitiveComponent))
  (Variables|Default|SetTurretMaterial _returnvalue)
  (bind _returnvalue_2 (Rendering|Material|CreateDynamicMaterialInstance (Variables|Default|GetBarrel) 1 "/Game/Art/3D/M_TeamColour.M_TeamColour" "None" :!class /Script/Engine.PrimitiveComponent))
  (Variables|Default|SetBarrelMaterial _returnvalue_2))

(event Collision|EventActorBeginOverlap
  (params (OtherActor :type Actor%20Object%20Reference))
  (|CallParentFunction OtherActor) ; This node is disabled and will not be called.\nDrag off pins to build functionality.
)

(event EventTick
  (params (DeltaSeconds :type Float%20%28single-precision%29))
  (|CallParentFunction DeltaSeconds) ; This node is disabled and will not be called.\nDrag off pins to build functionality.
)

(event EventPossessed
  (params (NewController :type Controller%20Object%20Reference))
  (bind _asbp_pc (Utilities|Casting|CastToBP_PC NewController))
  (CallFunction|ChangeTeamColour (Variables|/Game/Core/BP_PC.BP_PC_C|GetTeamColour _asbp_pc))
  (bind _returnvalue (UserInterface|CreateWidget "/Game/UI/BP_Test.BP_Test_C"))
  (UserInterface|Viewport|AddtoViewport _returnvalue 0))

(fn ConstructionScript
  (|CallParentFunction))