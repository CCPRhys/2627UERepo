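; BP_Plane is a flyable plane pawn with constant forward thrust and steerable pitch and roll.
; While it has a valid controller, Tick feeds full movement input along the actor's forward vector.
; The ApplyMovement event turns a vector input into local rotation, X for roll and Y for pitch, scaled by TurnSpeed and delta time, with no yaw.
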(event EventBeginPlay
  (|CallParentFunction) ; This node is disabled and will not be called.\nDrag off pins to build functionality.
)

(event Collision|EventActorBeginOverlap
  (params (OtherActor :type Actor%20Object%20Reference))
  (|CallParentFunction OtherActor) ; This node is disabled and will not be called.\nDrag off pins to build functionality.
)

(event EventTick
  (params (DeltaSeconds :type Float%20%28single-precision%29))
  (|CallParentFunction DeltaSeconds)
  (Utilities|IsValid (Pawn|GetController)
    (:Is%20Valid
      (Pawn|Input|AddMovementInput (Transformation|GetActorForwardVector) 1.0 false))))

(event EventApplyMovement
  (params (InVec :type Vector%202D%20Structure))
  (bind (_x _y) (Math|Vector2D|BreakVector2D InVec))
  (Transformation|AddActorLocalRotation (Math|Rotator|MakeRotator (* _x (Utilities|Time|GetWorldDeltaSeconds) (Variables|Default|GetTurnSpeed)) (* _y (Utilities|Time|GetWorldDeltaSeconds) (Variables|Default|GetTurnSpeed)) 0.0) false false))

(fn ConstructionScript
  (|CallParentFunction))